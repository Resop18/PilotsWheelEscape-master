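; PaperGameMode is a game mode that opens the game on an intro screen and tracks score and people statistics.
; On BeginPlay it adds the IntroScreen widget, disables player character input, shows the mouse cursor and pauses the game.
; Custom events increment counters for people saved, drowned and killed by gators, and add points to Score, truncating the float to whole numbers.
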(event `self.ReceiveBeginPlay`
  (bind _returnvalue (`GameplayStatics.GetPlayerController` 0))
  (bind _returnvalue_2 (`|CreateWidget` "/Game/HudStuff/IntroScreen.IntroScreen_C"))
  (`UserWidget.AddToViewport` _returnvalue_2 0)
  (`self.DisableInput` (`GameplayStatics.GetPlayerCharacter` 0) _returnvalue)
  (set `PlayerController.bShowMouseCursor` true _returnvalue)
  (`GameplayStatics.SetGamePaused` true))

(event `AddPoints`
  (params (AddScorePoints :type Integer))
  (set `self.Score` (`KismetMathLibrary.Conv_IntToDouble` (+ AddScorePoints (`KismetMathLibrary.FTrunc` (`self.Score`))))))

(event `AddSavedPeople`
  (`/Engine/EditorBlueprintResources/StandardMacros.IncrementInt` (`self.PEOPLESAVED`)))

(event `AddPeopleDrowned`
  (`/Engine/EditorBlueprintResources/StandardMacros.IncrementInt` (`self.PEOPLEDROWNED`)))

(event `AddDeathsByGator`
  (`/Engine/EditorBlueprintResources/StandardMacros.IncrementInt` (`self.DEATHBYGATOR`)))

(fn `UserConstructionScript`)