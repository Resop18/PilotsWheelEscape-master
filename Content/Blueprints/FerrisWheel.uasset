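; Ferris wheel actor with a tintable Cog sprite that moves when the CogForward event fires.
; CogForward plays a timeline that sets the Cog's relative location from two vector tracks, though the fixed zero Lerp alpha means only the first applies.
; The construction script stores the Cog's world location as EndLocation, applies it or zero as relative location depending on TestEndLocation, and applies FerrisWheelColor.
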(event `CogForward`
  (bind (_direction _newtrack_4 _newtrack_5) (`Timeline|Timeline_0` :!via `PlayFromStart`)
    (:`Update`
      (`SceneComponent.K2_SetRelativeLocation` (`self.Cog`) (`KismetMathLibrary.VLerp` _newtrack_4 _newtrack_5) false false))))

(fn `UserConstructionScript`
  (bind _cog (`self.Cog`))
  (bind _output_get (set `self.EndLocation` (`SceneComponent.K2_GetComponentLocation` (`self.Cog`))))
  (`SceneComponent.K2_SetRelativeLocation` _cog (`KismetMathLibrary.SelectVector` _output_get (0.0 0.0 0.0) (`self.TestEndLocation`)) false false)
  (`PaperSpriteComponent.SetSpriteColor` _cog (`self.FerrisWheelColor`)))