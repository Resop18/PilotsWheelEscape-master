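; 2D lift actor whose sprite shuttles between its origin and EndLocation, with a configurable travel time, stop delay and color.
; Once LiftForward is called, a timeline lerps the sprite and alternates direction after each delay.
; SafteyCollider overlaps by MyCharacter adjust active timeline playback, while SafteyBox overlaps destroy the character, add Points through PaperGameMode and respawn it at the player controller's transform.
; The construction script previews either endpoint via TestEndLocation.
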(event `self.ReceiveBeginPlay`
  (`TimelineComponent.SetPlayRate` (`self.LiftTimeline`) (/ 1.0 (`self.TravelTimeInSeconds`)))
  (set `self.TestEndLocation` true))

(event `LiftForward`
  (bind (_direction _driver) (`Timeline|LiftTimeline` :!via `PlayFromStart` :!label _label)
    (:`Update`
      (`SceneComponent.K2_SetRelativeLocation` (`self.LiftSprite`) (`KismetMathLibrary.VLerp` (0.0 0.0 0.0) (`self.EndLocation`) _driver) false false))
    (:`Finished`
      (`KismetSystemLibrary.Delay` (`self.StopDelay`))
      (switch `ETimelineDirection` _direction
        (:`Forward`
          (`self.LiftBackward`))
        (:`Backward`
          (`self.LiftForward`))))))

(event `LiftBackward`
  (goto _label :!via `ReverseFromEnd`))

(event `self.SafteyCollider.OnComponentBeginOverlap`
  (params (OverlappedComponent :type "PrimitiveComponent Object Reference") (OtherActor :type "Actor Object Reference") (OtherComp :type "PrimitiveComponent Object Reference") (OtherBodyIndex :type Integer) (bFromSweep :type Boolean) (SweepResult :type "HitResult Structure (by ref)"))
  (bind _lifttimeline (`self.LiftTimeline`))
  (cast `/Game/Blueprints/MyCharacter` OtherActor)
  (if (`ActorComponent.IsActive` _lifttimeline)
    (if (`TimelineComponent.IsPlaying` _lifttimeline)
      (goto _label)
      (else
        (goto _label :!via `Reverse`)))))

(event `self.SafteyBox.OnComponentBeginOverlap`
  (params (OverlappedComponent :type "PrimitiveComponent Object Reference") (OtherActor :type "Actor Object Reference") (OtherComp :type "PrimitiveComponent Object Reference") (OtherBodyIndex :type Integer) (bFromSweep :type Boolean) (SweepResult :type "HitResult Structure (by ref)"))
  (bind _returnvalue (`GameplayStatics.GetPlayerController` 0))
  (bind _asmy_character (cast `/Game/Blueprints/MyCharacter` OtherActor))
  (`Controller.UnPossess` _returnvalue)
  (`self.K2_DestroyActor` _asmy_character)
  (bind _aspaper_game_mode (cast `/Game/Blueprints/PaperGameMode` (`GameplayStatics.GetGameMode`)))
  (`/Game/Blueprints/PaperGameMode.AddPoints` _aspaper_game_mode (`self.Points`))
  (bind _returnvalue_2 (`|SpawnActorFromClass` "/Game/Blueprints/MyCharacter.MyCharacter_C" (`self.GetTransform` _returnvalue) "Undefined" "OverrideRootScale"))
  (`Controller.Possess` _returnvalue _returnvalue_2))

(fn `UserConstructionScript`
  (bind _liftsprite (`self.LiftSprite`))
  (`SceneComponent.K2_SetRelativeLocation` _liftsprite (`KismetMathLibrary.SelectVector` (`self.EndLocation`) (0.0 0.0 0.0) (`self.TestEndLocation`)) false false)
  (`PaperSpriteComponent.SetSpriteColor` _liftsprite (`self.LiftColor`)))