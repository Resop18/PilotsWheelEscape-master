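; OceanFloor is an actor that respawns the player's character when it touches the floor's Reset component.
; On overlap, it destroys the MyCharacter, unpossesses player controller 0, then spawns and possesses a new MyCharacter.
; The spawn transform comes from the player controller's own actor transform rather than a stored checkpoint or player start.
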(event `self.Reset.OnComponentBeginOverlap`
  (params (OverlappedComponent :type "PrimitiveComponent Object Reference") (OtherActor :type "Actor Object Reference") (OtherComp :type "PrimitiveComponent Object Reference") (OtherBodyIndex :type Integer) (bFromSweep :type Boolean) (SweepResult :type "HitResult Structure (by ref)"))
  (bind _returnvalue (`GameplayStatics.GetPlayerController` 0))
  (bind _asmy_character (cast `/Game/Blueprints/MyCharacter` OtherActor))
  (`self.K2_DestroyActor` _asmy_character)
  (`Controller.UnPossess` _returnvalue)
  (bind _returnvalue_2 (`|SpawnActorFromClass` "/Game/Blueprints/MyCharacter.MyCharacter_C" (`self.GetTransform` _returnvalue) "Undefined" "OverrideRootScale"))
  (`Controller.Possess` _returnvalue _returnvalue_2))

(fn `UserConstructionScript`
  (`parent.UserConstructionScript`))