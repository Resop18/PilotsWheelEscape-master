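; A spinning wheel actor that carries spawned platforms, with a player-adjustable rotation speed.
; BeginPlay spawns a PlatformsOnWheel at each WheelSprite socket named in MyArray, giving it the wheel's negated starting speed.
; Tick, behind a tiny Delay, slowly increases YawPerSecond and applies it as local pitch, despite the name.
; Speed Up and Down inputs change the wheel's speed in very unequal steps, without updating the platforms.
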(event `InputAction|Speed Down`
  (params (Key :type "Key Structure" :default "AnyKey"))
  (:`Pressed`
    (set `self.YawPerSecond` (+ (`self.YawPerSecond`) -10.0))))

(event `InputAction|Speed Up`
  (params (Key :type "Key Structure" :default "AnyKey"))
  (:`Pressed`
    (set `self.YawPerSecond` (+ (`self.YawPerSecond`) 1000.0))))

(event `self.ReceiveBeginPlay`
  (bind _yawpersecond (`self.YawPerSecond`))
  (for _array_element (`self.myArray`)
    (bind _returnvalue (`|SpawnActorFromClass` "/Game/Blueprints/PlatformsOnWheel.PlatformsOnWheel_C" (`KismetMathLibrary.MakeTransform` (0.0 0.0 0.0)) "Undefined" "OverrideRootScale"))
    (set `/Game/Blueprints/PlatformsOnWheel.YawPerSecond` (- _yawpersecond (* _yawpersecond 2.0)) _returnvalue)
    (`SceneComponent.K2_AttachToComponent` (`/Game/Blueprints/PlatformsOnWheel.root` _returnvalue) (`self.wheel_Sprite`) _array_element "KeepRelative" "KeepRelative" "KeepRelative" true)))

(event `self.ReceiveTick`
  (params (DeltaSeconds :type "Float (single-precision)"))
  (`KismetSystemLibrary.Delay` 1e-05)
  (bind _output_get (set `self.YawPerSecond` (+ (`self.YawPerSecond`) 0.0001)))
  (`self.K2_AddActorLocalRotation` (`KismetMathLibrary.MakeRotator` 0.0 (* DeltaSeconds _output_get))))

(fn `UserConstructionScript`)